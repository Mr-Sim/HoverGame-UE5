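; BP_Hover is a player-driven hover vehicle suspended on four corner hover components with repulsion and attraction springs.
; BeginPlay adds the input mapping and offsets each hover's range, damping and stiffness by shared tuning modifiers.
; Thrust, steer and boost inputs set BPMovementComponent targets, with thrust also updating its grounded state from front attraction hits.
; Tick toggles the lateral stabilizer and informs the hovers whenever all-four-corner grounding changes.
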(event Input|EnhancedActionEvents|EnhancedInputActionIA_Thrust
  (params (ActionValue :type Float%20%28double-precision%29) (ElapsedSeconds :type Float%20%28double-precision%29) (TriggeredSeconds :type Float%20%28double-precision%29) (InputAction :type Input%20Action%20Object%20Reference :default "/Game/04-Inputs/Actions/IA_Thrust.IA_Thrust"))
  (bind _bp_movementcomponent (Variables|Default|GetBP_MovementComponent))
  (:Triggered
    (bind _grounded (CallFunction|CheckFrontGrounded))
    (Variables|/Game/01-Blueprints/Components/BP_MovementComponent.BP_MovementComponent_C|SetIsGrounded _bp_movementcomponent _grounded)
    (Variables|/Game/01-Blueprints/Components/BP_MovementComponent.BP_MovementComponent_C|SetTargetSpeed _bp_movementcomponent (* ActionValue (Variables|Default|GetMaxSpeed) (Variables|Default|GetBoostMultiplier)))
    (Development|PrintText "THRUST" true true "(R=0.221021,G=0.000000,B=1.000000,A=1.000000)" 0.01 "0.1"))
  (:Completed
    (Variables|/Game/01-Blueprints/Components/BP_MovementComponent.BP_MovementComponent_C|SetTargetSpeed _bp_movementcomponent 0.0)))

(event Input|EnhancedActionEvents|EnhancedInputActionIA_Steer
  (params (ActionValue :type Float%20%28double-precision%29) (ElapsedSeconds :type Float%20%28double-precision%29) (TriggeredSeconds :type Float%20%28double-precision%29) (InputAction :type Input%20Action%20Object%20Reference :default "/Game/04-Inputs/Actions/IA_Steer.IA_Steer"))
  (bind _bp_movementcomponent (Variables|Default|GetBP_MovementComponent))
  (:Triggered
    (Variables|/Game/01-Blueprints/Components/BP_MovementComponent.BP_MovementComponent_C|SetTargetAngularSpeed _bp_movementcomponent (* ActionValue (Variables|Default|GetMaxAngularSpeed)))
    (Development|PrintText "STEER" true true "(R=0.221021,G=0.000000,B=1.000000,A=1.000000)" 0.01 "1"))
  (:Completed
    (Variables|/Game/01-Blueprints/Components/BP_MovementComponent.BP_MovementComponent_C|SetTargetAngularSpeed _bp_movementcomponent 0.0)))

(event Input|EnhancedActionEvents|EnhancedInputActionIA_Boost
  (params (ActionValue :type Boolean) (ElapsedSeconds :type Float%20%28double-precision%29) (TriggeredSeconds :type Float%20%28double-precision%29) (InputAction :type Input%20Action%20Object%20Reference :default "/Game/04-Inputs/Actions/IA_Boost.IA_Boost"))
  (:Started
    (Variables|Default|SetBoostMultiplier (Variables|Default|GetBoostFactor)))
  (:Completed
    (Variables|Default|SetBoostMultiplier 1.0)))

(event EventBeginPlay
  (bind _returnvalue (Game|GetPlayerController 0))
  (bind _returnvalue_2 (PlayerController|LocalPlayerSubsystems|GetEnhancedInputLocalPlayerSubsystem _returnvalue))
  (Utilities|IsValid _returnvalue_2
    (:Is%20Valid
      (Input|AddMappingContext _returnvalue_2 "/Game/04-Inputs/IMC_Hover.IMC_Hover" 0 "(bIgnoreAllPressedKeysUntilRelease=True,bForceImmediately=False,bNotifyUserSettings=False)")
      (Utilities|FlowControl|Sequence
        (:then_0
          (bind _output_get (Variables|Default|SetHOVERS (Utilities|Array|MakeArray (Variables|Default|GetFrontLeftHoverComponent) (Variables|Default|GetRearLeftHoverComponent) (Variables|Default|GetFrontRightHoverComponent) (Variables|Default|GetRearRightHoverComponent))))
          (for _array_element _output_get
            (Utilities|FlowControl|Sequence
              (:then_0
                (Variables|/Game/01-Blueprints/Components/BP_HoverComponent.BP_HoverComponent_C|SetRep_Range _array_element (+ (Variables|Default|GetHoverHeightModifier) (Variables|/Game/01-Blueprints/Components/BP_HoverComponent.BP_HoverComponent_C|GetRep_Range _array_element)))
                (Variables|/Game/01-Blueprints/Components/BP_HoverComponent.BP_HoverComponent_C|SetAttr_Range _array_element (+ (Variables|Default|GetHoverHeightModifier) (Variables|/Game/01-Blueprints/Components/BP_HoverComponent.BP_HoverComponent_C|GetAttr_Range _array_element))))
              (:then_1
                (Variables|/Game/01-Blueprints/Components/BP_HoverComponent.BP_HoverComponent_C|SetRep_Damp _array_element (+ (Variables|Default|GetDampingModifier) (Variables|/Game/01-Blueprints/Components/BP_HoverComponent.BP_HoverComponent_C|GetRep_Damp _array_element)))
                (Variables|/Game/01-Blueprints/Components/BP_HoverComponent.BP_HoverComponent_C|SetAttr_Damp _array_element (+ (Variables|Default|GetAttrDampingModifier) (Variables|/Game/01-Blueprints/Components/BP_HoverComponent.BP_HoverComponent_C|GetAttr_Damp _array_element))))
              (:then_2
                (Variables|/Game/01-Blueprints/Components/BP_HoverComponent.BP_HoverComponent_C|SetRep_Stiff _array_element (+ (Variables|Default|GetStiffnessModifier) (Variables|/Game/01-Blueprints/Components/BP_HoverComponent.BP_HoverComponent_C|GetRep_Stiff _array_element)))
                (Variables|/Game/01-Blueprints/Components/BP_HoverComponent.BP_HoverComponent_C|SetAttr_Stiff _array_element (+ (Variables|Default|GetAttrStiffnessModifier) (Variables|/Game/01-Blueprints/Components/BP_HoverComponent.BP_HoverComponent_C|GetAttr_Stiff _array_element))))
              (:then_3))))))
    (:Is%20Not%20Valid
      (Development|PrintString "Enhanced Input Local System not valid"))))

(event EventTick
  (params (DeltaSeconds :type Float%20%28single-precision%29))
  (bind _bp_lateralstabilizer (Variables|Default|GetBP_LateralStabilizer))
  (Utilities|FlowControl|Sequence
    (:then_0
      (bind _grounded (CallFunction|CheckFullGrounded))
      (if (!= _grounded (Variables|Default|GetWheels%20Grounded))
        (bind _output_get (Variables|Default|SetWheels%20Grounded _grounded))
        (if _output_get
          (Components|Activation|Activate _bp_lateralstabilizer true)
          (else
            (Components|Activation|Deactivate _bp_lateralstabilizer)))
        (for _array_element (Variables|Default|GetHOVERS)
          (Variables|/Game/01-Blueprints/Components/BP_HoverComponent.BP_HoverComponent_C|SetWheelsGrounded _array_element _output_get))))))

(fn ConstructionScript)

(fn CheckGrounded
  (return (Math|Boolean|ORBoolean (Variables|/Game/01-Blueprints/Components/BP_HoverComponent.BP_HoverComponent_C|GetAttr_Hit (Variables|Default|GetFrontLeftHoverComponent)) (Variables|/Game/01-Blueprints/Components/BP_HoverComponent.BP_HoverComponent_C|GetAttr_Hit (Variables|Default|GetRearLeftHoverComponent)) (Variables|/Game/01-Blueprints/Components/BP_HoverComponent.BP_HoverComponent_C|GetAttr_Hit (Variables|Default|GetFrontRightHoverComponent)) (Variables|/Game/01-Blueprints/Components/BP_HoverComponent.BP_HoverComponent_C|GetAttr_Hit (Variables|Default|GetRearRightHoverComponent)))))

(fn CheckFrontGrounded
  (return (or (Variables|/Game/01-Blueprints/Components/BP_HoverComponent.BP_HoverComponent_C|GetAttr_Hit (Variables|Default|GetFrontLeftHoverComponent)) (Variables|/Game/01-Blueprints/Components/BP_HoverComponent.BP_HoverComponent_C|GetAttr_Hit (Variables|Default|GetFrontRightHoverComponent)))))

(fn CheckFullGrounded
  (return (Math|Boolean|ANDBoolean (Variables|/Game/01-Blueprints/Components/BP_HoverComponent.BP_HoverComponent_C|GetAttr_Hit (Variables|Default|GetFrontLeftHoverComponent)) (Variables|/Game/01-Blueprints/Components/BP_HoverComponent.BP_HoverComponent_C|GetAttr_Hit (Variables|Default|GetRearLeftHoverComponent)) (Variables|/Game/01-Blueprints/Components/BP_HoverComponent.BP_HoverComponent_C|GetAttr_Hit (Variables|Default|GetFrontRightHoverComponent)) (Variables|/Game/01-Blueprints/Components/BP_HoverComponent.BP_HoverComponent_C|GetAttr_Hit (Variables|Default|GetRearRightHoverComponent)))))