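; Spline-based actor that tiles a chosen static mesh along its spline, deforming each copy to follow the curve.
; The construction script, skipped without a valid mesh, derives segment length from the mesh's X bounds and divides the spline length by it.
; It adds a collision-enabled, X-forward spline mesh component per segment, using local spline positions and tangents clamped to segment length.
; The event graph has no active logic.
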(event EventBeginPlay)

(event Collision|EventActorBeginOverlap
  (params (OtherActor :type Actor%20Object%20Reference)))

(event EventTick
  (params (DeltaSeconds :type Float%20%28single-precision%29)))

(fn ConstructionScript
  (bind _spline (Variables|Default|GetSpline))
  (bind _spline_2 (Variables|Default|GetSpline))
  (bind _mesh (Variables|Default|GetMesh)
    (:then
      (bind _output_get (Variables|Default|SetXlength (.x (+ (Math|Vector|VectorGetAbs (.Min (Utilities|Struct|BreakBox (StaticMesh|GetBoundingBox _mesh)))) (Math|Vector|VectorGetAbs (.Max (Utilities|Struct|BreakBox (StaticMesh|GetBoundingBox _mesh))))))))
      (for _index (range 0 (Math|Float|Truncate (/ (Spline|GetSplineLength (Variables|Default|GetSpline)) _output_get)))
        (bind _returnvalue (AddComponent|AddSplineMeshComponent false))
        (Collision|SetCollisionEnabled _returnvalue "QueryAndPhysics")
        (SplineMesh|SetForwardAxis _returnvalue "X" true)
        (Components|StaticMesh|SetStaticMesh _returnvalue (Variables|Default|GetMesh))
        (SplineMesh|SetStartandEnd _returnvalue (Spline|GetLocationatDistanceAlongSpline _spline_2 (* _index (Variables|Default|GetXlength)) "Local") (Math|Vector|ClampVectorSize (Spline|GetTangentatDistanceAlongSpline _spline_2 (* _index (Variables|Default|GetXlength)) "Local") 0.0 (Variables|Default|GetXlength)) (Spline|GetLocationatDistanceAlongSpline _spline (* (+ _index 1) (Variables|Default|GetXlength)) "Local") (Math|Vector|ClampVectorSize (Spline|GetTangentatDistanceAlongSpline _spline (* (+ _index 1) (Variables|Default|GetXlength)) "Local") 0.0 (Variables|Default|GetXlength)) true :!class /Script/Engine.SplineMeshComponent)))
    (:else)))