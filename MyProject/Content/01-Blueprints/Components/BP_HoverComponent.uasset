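; Hover component that applies spring-damper suspension forces at its own location to the owner's physics-simulated root primitive.
; Each tick, a downward line trace over the attraction range drives a force along the component's up vector, turning into a downward pull when WheelsGrounded is set.
; When that trace hits, a second trace adds a repulsion force.
; Both derive force from normalized compression and its rate of change, with separate stiffness and damping.
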(event EventBeginPlay
  (bind _asprimitive_component (Utilities|Casting|CastToPrimitiveComponent (Variables|/Script/Engine.Actor|GetRootComponent (Components|GetOwner)))
    (:then
      (bind _output_get (Variables|Default|SetRefToVehicle _asprimitive_component))
      (if (not (Physics|IsSimulatingPhysics _output_get "None"))
        (Variables|Default|SetRefToVehicle 0)
        (Development|PrintText "BP_Component cannot work on non physical object" true true "(R=1.000000,G=0.238000,B=0.000000,A=1.000000)" 5.0)))
    (:CastFailed
      (Development|PrintText "CAST TO PRIMITIVE TARGET FAILED : BP_HoverComponent" true true "(R=1.000000,G=0.005365,B=0.000000,A=1.000000)" 5.0)
      (Components|DestroyComponent))))

(event EventTick
  (params (DeltaSeconds :type Float%20%28single-precision%29))
  (Variables|Default|GetRefToVehicle
    (:then
      (Utilities|FlowControl|Sequence
        (:then_0
          ;[0.2163 0.6931 1] Attraction
          (bind (_outhit _hit) (CallFunction|RayCast (Variables|Default|GetAttr_Range) true "(R=0.000000,G=0.011881,B=1.000000,A=1.000000)" "(R=0.033181,G=0.000000,B=1.000000,A=1.000000)"))
          (bind _output_get (Variables|Default|SetAttr_Hit _hit))
          (if _output_get
            (bind (_hoverforce _newcompression) (CallFunction|CalculateForce (Variables|Default|GetAttr_Range) (.Distance (Collision|BreakHitResult _outhit)) (Variables|Default|GetAttr_PreviousCompressionRange) (Variables|Default|GetAttr_Stiff) (Variables|Default|GetAttr_Damp) (Variables|Default|GetWheelsGrounded)))
            (bind _output_get_2 (Variables|Default|SetAttr_Force (Math|Float|Lerp (Variables|Default|GetAttr_Force) _hoverforce 1.0)))
            (Variables|Default|SetAttr_PreviousCompressionRange _newcompression)
            (Class|PrimitiveComponent|AddForceatLocation (Variables|Default|GetRefToVehicle) (* _output_get_2 (Math|Vector|GetUpVector)) (Transformation|GetWorldLocation) "None")))
        (:then_1
          ;[1 0.4862 0.1458] Repultion
          (if (Variables|Default|GetAttr_Hit)
            (bind (_outhit_2 _hit_2) (CallFunction|RayCast (Variables|Default|GetRep_Range) true "(R=1.000000,G=0.000000,B=0.464126,A=1.000000)" "(R=1.000000,G=0.382568,B=0.000000,A=1.000000)"))
            (bind _output_get_3 (Variables|Default|SetRep_Hit _hit_2))
            (if _output_get_3
              (bind (_hoverforce_2 _newcompression_2) (CallFunction|CalculateForce (Variables|Default|GetRep_Range) (.Distance (Collision|BreakHitResult _outhit_2)) (Variables|Default|GetRep_PreviousCompression) (Variables|Default|GetRep_Stiff) (Variables|Default|GetRep_Damp) false))
              (bind _output_get_4 (Variables|Default|SetRep_Force _hoverforce_2))
              (Variables|Default|SetRep_PreviousCompression _newcompression_2)
              (Class|PrimitiveComponent|AddForceatLocation (Variables|Default|GetRefToVehicle) (* _output_get_4 (Math|Vector|GetUpVector)) (Transformation|GetWorldLocation) "None"))))))
    (:else
      (Development|PrintString "Nope Hover"))))

(fn RayCast
  (params (Distance :type Float%20%28double-precision%29) (DrawRay :type Boolean) (TraceColor :type Linear%20Color%20Structure :default "(R=1.000000,G=0.000000,B=0.000000,A=1.000000)") (Trace%20Hit%20Color :type Linear%20Color%20Structure :default "(R=0.272618,G=1.000000,B=0.000000,A=1.000000)"))
  (bind _returnvalue (Transformation|GetWorldLocation))
  (bind (_outhit _returnvalue_2) (Collision|LineTraceByChannel _returnvalue (- _returnvalue (* Distance (Math|Vector|GetUpVector))) "TraceTypeQuery1" false (Utilities|Array|MakeArray (Components|GetOwner)) (select DrawRay "ForOneFrame" "None") true TraceColor Trace%20Hit%20Color))
  (return _outhit _returnvalue_2))

(fn CalculateForce
  (params (Range :type Float%20%28double-precision%29) (Distance :type Float%20%28double-precision%29) (PreviousCompression :type Float%20%28double-precision%29) (Stiffness :type Float%20%28double-precision%29) (Damping :type Float%20%28double-precision%29) (InvertCompression :type Boolean))
  (bind _returnvalue (Math|Conversions|ToFloat(Boolean) InvertCompression))
  (bind _returnvalue_2 (- 1.0 _returnvalue))
  (bind _returnvalue_3 (* Range _returnvalue_2))
  (bind _returnvalue_4 (- _returnvalue_3 Distance))
  (bind _returnvalue_5 (/ _returnvalue_4 Range))
  (return (+ (* (/ (- _returnvalue_5 PreviousCompression) (Utilities|Time|GetWorldDeltaSeconds)) Damping) (* _returnvalue_5 Stiffness)) _returnvalue_5))