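; Hover scene component for physics-driven vehicles, apparently an unfinished composite of attraction and repulsion springs.
; BeginPlay caches the owner's root primitive, rejecting it unless it simulates physics.
; DoRayCast traces along local down for spring distances, and CalculateForce computes spring-damper force.
; Tick applies no force: both force chains are disconnected, DoRayCast is never called and ApplyForce is empty.
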(event EventBeginPlay
  (bind _asprimitive_component (Utilities|Casting|CastToPrimitiveComponent (Variables|/Script/Engine.Actor|GetRootComponent (Components|GetOwner)))
    (:then
      (bind _output_get (Variables|Default|SetRefToVehicle _asprimitive_component))
      (if (not (Physics|IsSimulatingPhysics _output_get "None"))
        (Variables|Default|SetRefToVehicle 0)
        (Development|PrintText "BP_Component cannot work on non physical object" true true "(R=1.000000,G=0.238000,B=0.000000,A=1.000000)" 5.0)))
    (:CastFailed
      (Development|PrintText "CAST TO PRIMITIVE TARGET FAILED : BP_HoverComponent" true true "(R=1.000000,G=0.005365,B=0.000000,A=1.000000)" 5.0)
      (Components|DestroyComponent))))

(event EventTick
  (params (DeltaSeconds :type Float%20%28single-precision%29))
  (Variables|Default|GetRefToVehicle
    (:then
      (Utilities|FlowControl|Sequence
        (:then_1
          ;[1 0.4862 0.1458] Repultion
          (if (Variables|Default|GetAttr_Hit)
            _))))
    (:else
      (Development|PrintString "Nope Hover"))))

(fn DoRayCast
  (params (DrawRay :type Boolean) (TraceColor :type Linear%20Color%20Structure :default "(R=1.000000,G=0.000000,B=0.000000,A=1.000000)"))
  (bind _returnvalue (Transformation|GetWorldLocation))
  (bind (_outhit _returnvalue_2) (Collision|LineTraceByChannel _returnvalue (- _returnvalue (* (Variables|Default|GetAttr_Range) (Math|Vector|GetUpVector))) "TraceTypeQuery1" false (Utilities|Array|MakeArray (Components|GetOwner)) (select DrawRay "ForOneFrame" "None") true TraceColor))
  (Variables|Default|SetAttr_Hit _returnvalue_2)
  (bind _output_get (Variables|Default|SetAttr_Dist (.Distance (Collision|BreakHitResult _outhit))))
  (Variables|Default|SetRep_Dist (Math|Float|Clamp(Float) _output_get 0.0 (Variables|Default|GetRep_Range))))

(fn CalculateForce
  (params (Compression :type Float%20%28double-precision%29) (PreviousCompression :type Float%20%28double-precision%29) (Stiffness :type Float%20%28double-precision%29) (Damping :type Float%20%28double-precision%29))
  (return (+ (* (/ (- Compression PreviousCompression) (Utilities|Time|GetWorldDeltaSeconds)) Damping) (* Compression Stiffness))))

(fn ApplyForce)