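; Component that manages a set of hovers on a physics-simulated vehicle, using the owner's primitive root as the vehicle body.
; BeginPlay rejects non-simulating roots and destroys the component if the root is not a primitive.
; Each Tick ray-casts every hover with debug drawing and sums compression from its attraction distance and range.
; No force is applied here, and the inverted compression formula reduces to -1 for any nonzero distance.
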(event EventBeginPlay
  (bind _asprimitive_component (Utilities|Casting|CastToPrimitiveComponent (Variables|/Script/Engine.Actor|GetRootComponent (Components|GetOwner)))
    (:then
      (bind _output_get (Variables|Default|SetRefToVehicle _asprimitive_component))
      (if (not (Physics|IsSimulatingPhysics _output_get "None"))
        (Variables|Default|SetRefToVehicle 0)
        (Development|PrintText "BP_Component cannot work on non physical object" true true "(R=1.000000,G=0.238000,B=0.000000,A=1.000000)" 5.0)))
    (:CastFailed
      (Development|PrintText "CAST TO PRIMITIVE TARGET FAILED : BP_HoverComponent" true true "(R=1.000000,G=0.005365,B=0.000000,A=1.000000)" 5.0)
      (Components|DestroyComponent))))

(event EventTick
  (params (DeltaSeconds :type Float%20%28single-precision%29))
  (Variables|Default|GetRefToVehicle
    (:then
      (Variables|Default|SetAttr_PreviousCompression 0.0)
      (Variables|Default|SetRep_PreviousCompression 0.0)
      (Utilities|FlowControl|Sequence
        (:then_0
          (for _array_element (Variables|Default|GetHovers)
            (Default|DoRayCast _array_element true "(R=0.000000,G=0.109944,B=1.000000,A=1.000000)")
            (Utilities|FlowControl|Sequence
              (:then_0
                (bind _compression (CallFunction|CalculateCompression (Variables|/Game/01-Blueprints/Components/BP_HoverCompositeComponent.BP_HoverCompositeComponent_C|GetAttr_Dist _array_element) (Variables|/Game/01-Blueprints/Components/BP_HoverCompositeComponent.BP_HoverCompositeComponent_C|GetAttr_Range _array_element) true))
                (Variables|Default|SetAttr_PreviousCompression (+ _compression (Variables|Default|GetAttr_PreviousCompression)))))))))
    (:else)))

(fn CalculateCompression
  (params (Distance :type Float%20%28double-precision%29) (Range :type Float%20%28double-precision%29) (InvertCompression :type Boolean))
  (return (/ (- (* Range (- 1.0 (Math|Conversions|ToFloat(Boolean) InvertCompression))) Distance) Distance)))