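; BP_LateralStabilizer is a component that damps sideways sliding on a physics-simulated vehicle.
; On BeginPlay it caches the owner's root primitive, clearing it if not simulating physics and destroying itself if the cast fails.
; Each tick it projects linear velocity onto the forward vector and applies an opposing force scaled by LateralDamping.
; The forward vector serves as the lateral axis because the model is not oriented on X.
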(event EventBeginPlay
  (bind _asprimitive_component (Utilities|Casting|CastToPrimitiveComponent (Variables|/Script/Engine.Actor|GetRootComponent (Components|GetOwner)))
    (:then
      (bind _output_get (Variables|Default|SetReftoVehicle _asprimitive_component))
      (if (not (Physics|IsSimulatingPhysics _output_get "None"))
        (Variables|Default|SetReftoVehicle 0)
        (Development|PrintText "BP_Component cannot work on non physical object" true true "(R=1.000000,G=0.238000,B=0.000000,A=1.000000)" 5.0)))
    (:CastFailed
      (Development|PrintText "CAST TO PRIMITIVE TARGET FAILED : BP_LateralStabilizer" true true "(R=1.000000,G=0.005365,B=0.000000,A=1.000000)" 5.0)
      (Components|DestroyComponent))))

(event EventTick
  (params (DeltaSeconds :type Float%20%28single-precision%29))
  (bind _reftovehicle (Variables|Default|GetReftoVehicle)
    (:then
      (bind _returnvalue (Physics|GetPhysicsLinearVelocity _reftovehicle "None"))
      (Physics|AddForce (Variables|Default|GetReftoVehicle) (* (Math|Vector|DotProduct _returnvalue (Math|Vector|GetForwardVector _reftovehicle)) -1.0 (Variables|Default|GetLateralDamping) (Math|Vector|GetForwardVector _reftovehicle)) "None" false))
    (:else
      (Development|PrintString "Nope Lateral Stabilizer"))))