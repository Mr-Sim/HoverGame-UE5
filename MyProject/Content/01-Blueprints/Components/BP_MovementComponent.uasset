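; BP_MovementComponent is a physics-based vehicle movement component that drives its owner's root primitive toward target linear and angular speeds.
; BeginPlay caches the root, clearing it if not simulating physics and destroying the component if it is not a primitive.
; While grounded, Tick applies proportional force along the right vector, used as the travel axis, and torque around the up vector, scaled by each speed error.
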(event EventBeginPlay
  (bind _asprimitive_component (Utilities|Casting|CastToPrimitiveComponent (Variables|/Script/Engine.Actor|GetRootComponent (Components|GetOwner)))
    (:then
      (bind _output_get (Variables|Default|SetRefToVehicle _asprimitive_component))
      (if (not (Physics|IsSimulatingPhysics _output_get "None"))
        (Variables|Default|SetRefToVehicle 0)
        (Development|PrintText "BP_Component cannot work on non physical object" true true "(R=1.000000,G=0.238000,B=0.000000,A=1.000000)" 5.0)))
    (:CastFailed
      (Development|PrintText "CAST TO PRIMITIVE TARGET FAILED : BP_MovementComponent" true true "(R=1.000000,G=0.005365,B=0.000000,A=1.000000)" 5.0)
      (Components|DestroyComponent))))

(event EventTick
  (params (DeltaSeconds :type Float%20%28single-precision%29))
  (bind _reftovehicle (Variables|Default|GetRefToVehicle))
  (bind _reftovehicle_2 (Variables|Default|GetRefToVehicle))
  (bind _reftovehicle_3 (Variables|Default|GetRefToVehicle))
  (if (Variables|Default|GetIsGrounded)
    (bind _reftovehicle_4 (Variables|Default|GetRefToVehicle)
      (:then
        (Utilities|FlowControl|Sequence
          (:then_0
            (bind _returnvalue (Physics|GetPhysicsLinearVelocity _reftovehicle_4 "None"))
            (bind _output_get (Variables|Default|SetCurrentSpeed (Math|Vector|DotProduct _returnvalue (Math|Vector|GetRightVector _reftovehicle_4))))
            (Physics|AddForce _reftovehicle_2 (* (Math|Vector|GetRightVector _reftovehicle_2) (- (Variables|Default|GetTargetSpeed) _output_get) (Variables|Default|GetSpeedToForceFactor)) "None" false))
          (:then_1
            (bind _output_get_2 (Variables|Default|SetCurrentAngularSpeed (Math|Vector|DotProduct (Physics|GetPhysicsAngularVelocityinDegrees _reftovehicle "None") (Math|Vector|GetUpVector _reftovehicle))))
            (Class|PrimitiveComponent|AddTorqueinDegrees _reftovehicle_3 (* (Math|Vector|GetUpVector _reftovehicle_3) (- (Variables|Default|GetTargetAngularSpeed) _output_get_2) (Variables|Default|GetAngularSpeedToForceFactor)) "None" false))))
      (:else
        (Development|PrintString "Nope Movement")))))