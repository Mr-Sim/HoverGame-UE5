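; BP_CheckpointBase is a race checkpoint that reports when a BP_Hover passes through it while it is the next checkpoint.
; Actor overlap casts to BP_Hover, checks IsNextCheckpoint, then calls the CheckpointCleared dispatcher.
; Activate and Deactivate set that flag and both toggle the PointLight's visibility rather than setting it explicitly, so the light depends on the calls alternating.
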(event EventBeginPlay)

(event Collision|EventActorBeginOverlap
  (params (OtherActor :type Actor%20Object%20Reference))
  (Utilities|Casting|CastToBP_Hover OtherActor)
  (if (Variables|Default|GetIsNextCheckpoint)
    (Default|CallCheckpointCleared)))

(event EventTick
  (params (DeltaSeconds :type Float%20%28single-precision%29)))

(fn ConstructionScript)

(fn Activate
  (Variables|Default|SetIsNextCheckpoint true)
  (Rendering|ToggleVisibility (Variables|Default|GetPointLight) false))

(fn Deactivate
  (Variables|Default|SetIsNextCheckpoint false)
  (Rendering|ToggleVisibility (Variables|Default|GetPointLight) false))